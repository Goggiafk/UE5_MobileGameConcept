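; BP_Stickman is a stickman actor that destroys itself and an actor it collides with when their tags differ.
; On a capsule hit with a tagged actor, it stores that actor, switches on its first tag, and compares both actors' second tags, apparently as a team marker.
; A mismatch calls DestroyBoth, which removes both actors if the stored one is still valid.
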(event OnComponentHit(Capsule)
  (params (HitComponent :type Primitive%20Component%20Object%20Reference) (OtherActor :type Actor%20Object%20Reference) (OtherComp :type Primitive%20Component%20Object%20Reference) (NormalImpulse :type Vector :default "0, 0, 0") (Hit :type Hit%20Result%20Structure%20%28by%20ref%29))
  (Utilities|IsValid OtherActor
    (:Is%20Valid
      (if (Utilities|Array|IsNotEmpty (Variables|/Script/Engine.Actor|GetTags OtherActor))
        (Variables|Default|SetOther%20Actor OtherActor)
        (switch name (Utilities|Array|Get(acopy) (Variables|/Script/Engine.Actor|GetTags (Variables|Default|GetOther%20Actor)))
          (:Stickman
            (if (!= (Utilities|Array|Get(acopy) (Variables|/Script/Engine.Actor|GetTags (Variables|Default|GetOther%20Actor)) 1) (Utilities|Array|Get(acopy) (Variables|Actor|GetTags self) 1))
              (CallFunction|DestroyBoth))))))))

(event Custom|DestroyBoth
  (bind _other_actor (Variables|Default|GetOther%20Actor))
  (Utilities|IsValid _other_actor
    (:Is%20Valid
      (Actor|DestroyActor _other_actor)
      (Actor|DestroyActor self))))

(event EventDestroyed)

(fn ConstructionScript)