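; BP_Wall1 is a destructible wall that kills stickmen on contact and loses one health for each.
; A widget shows the remaining health, set on BeginPlay and updated on every hit.
; Hits from Player-tagged actors call Die on the stickman, play a sound and a timeline scale punch on the skeletal mesh.
; When health drops below one, the wall destroys itself after a short delay.
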(event OnComponentHit(StaticMesh)
  (params (HitComponent :type Primitive%20Component%20Object%20Reference) (OtherActor :type Actor%20Object%20Reference) (OtherComp :type Primitive%20Component%20Object%20Reference) (NormalImpulse :type Vector :default "0, 0, 0") (Hit :type Hit%20Result%20Structure%20%28by%20ref%29))
  (Utilities|IsValid OtherActor
    (:Is%20Valid
      (if (Utilities|Array|IsNotEmpty (Variables|/Script/Engine.Actor|GetTags OtherActor))
        (Variables|Default|SetOther%20Actor OtherActor)
        (switch name (Utilities|Array|Get(acopy) (Variables|/Script/Engine.Actor|GetTags (Variables|Default|GetOther%20Actor)))
          (:Stickman
            (if (Actor|ActorHasTag (Variables|Default|GetOther%20Actor) "Player")
              (bind _asbp_stickman (Utilities|Casting|CastToBP_Stickman (Variables|Default|GetOther%20Actor)))
              (Default|Die _asbp_stickman)
              (Variables|Default|SetOther%20Actor 0)
              (bind _result (Math|Integer|DecrementInt (Variables|Default|GetHealth))
                (:%20%20
                  (Default|SetCountText (Variables|Default|GetCountWidget) _result false)
                  (CallFunction|PlayHitAnimation)
                  (Audio|PlaySound2D (Variables|/Game/Blueprints/BP_GameTuning.BP_GameTuning_C|GetWallHitSound (Variables|Default|GetGameSeettings)) 1.0 1.0 0.0 0 0)
                  (if (< _result 1)
                    (Utilities|FlowControl|Delay 0.2)
                    (Actor|DestroyActor self)))))))))))

(event Custom|PlayHitAnimation
  (bind _scale (Timeline|Timeline PlayFromStart)
    (:Update
      (Transformation|SetRelativeScale3D (Variables|Default|GetSkeletalMesh) (+ (Variables|Default|GetCachedScale) _scale)))))

(event EventBeginPlay
  (bind _aswbp_count (Utilities|Casting|CastToWBP_Count (UserInterface|GetWidget (Variables|Default|GetWidget))))
  (bind _output_get (Variables|Default|SetCountWidget _aswbp_count))
  (Default|SetCountText _output_get (Variables|Default|GetHealth) false)
  (Variables|Default|SetCachedScale (Variables|/Script/Engine.SceneComponent|GetRelativeScale3D (Variables|Default|GetSkeletalMesh))))

(fn ConstructionScript
  (Rendering|SetCastShadow (Variables|Default|GetWidget) false))