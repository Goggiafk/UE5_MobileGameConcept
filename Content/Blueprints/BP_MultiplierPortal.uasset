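; A multiplier portal that turns each player stickman entering it into a Multiplier number of new stickmen.
; On BeginPlay it writes the multiplier to its count widget and colors the trigger area good or bad by the value's sign.
; On overlap it destroys the stickman, then asks the StickmenManager to spawn replacements slightly ahead of its saved transform.
; Replacements are tagged with the portal's name, so the same portal never multiplies them again.
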(event Collision|EventActorBeginOverlap
  (params (OtherActor :type Actor%20Object%20Reference))
  (bind _stickmenmanager (Variables|Default|GetStickmenManager))
  (Utilities|IsValid OtherActor
    (:Is%20Valid
      (if (Utilities|Array|IsNotEmpty (Variables|/Script/Engine.Actor|GetTags OtherActor))
        (Variables|Default|SetOther%20Actor OtherActor)
        (switch name (Utilities|Array|Get(acopy) (Variables|/Script/Engine.Actor|GetTags (Variables|Default|GetOther%20Actor)))
          (:Stickman
            (if (Actor|ActorHasTag (Variables|Default|GetOther%20Actor) "Player")
              (if (not (Actor|ActorHasTag (Variables|Default|GetOther%20Actor) (Utilities|String|StringToName (Utilities|GetObjectName self))))
                (Utilities|FlowControl|Sequence
                  (:then_0
                    (Utilities|IsValid (Variables|Default|GetOther%20Actor)
                      (:Is%20Valid
                        (Variables|Default|SetSavedLocation (Transformation|GetActorTransform (Variables|Default|GetOther%20Actor)))
                        (Variables|Default|SetSavedForwardVector (Transformation|GetActorForwardVector (Variables|Default|GetOther%20Actor)))
                        (Actor|DestroyActor (Variables|Default|GetOther%20Actor))
                        (Variables|Default|SetOther%20Actor 0))))
                  (:then_1
                    (for _index (range 1 (Variables|Default|GetMultiplier))
                      (Utilities|IsValid _stickmenmanager
                        (:Is%20Valid
                          (Default|SpawnStickman _stickmenmanager (Math|Transform|MakeTransform (+ (.location (Variables|Default|GetSavedLocation)) (* (Variables|Default|GetSavedForwardVector) 1e+01)) (.rotation (Variables|Default|GetSavedLocation)) (.scale (Variables|Default|GetSavedLocation))) false (Utilities|String|StringToName (Utilities|GetObjectName self))))))))))))))))

(event EventBeginPlay
  (bind _gamesettings (Variables|Default|GetGameSettings))
  (Utilities|FlowControl|Sequence
    (:then_0
      (bind _aswbp_count (Utilities|Casting|CastToWBP_Count (UserInterface|GetWidget (Variables|Default|GetWidget))))
      (Default|SetCountText _aswbp_count (Variables|Default|GetMultiplier) true))
    (:then_1
      (bind _returnvalue (Actor|GetActorOfClass "/Game/Blueprints/BP_StickmenManager.BP_StickmenManager_C"))
      (Variables|Default|SetStickmenManager _returnvalue))
    (:then_2
      (Rendering|Material|SetVectorParameterValueonMaterials (Variables|Default|GetTriggerArea) "Color" (Math|Conversions|ToVector(LinearColor) (select (> (Variables|Default|GetMultiplier) 0) (Variables|/Game/Blueprints/BP_GameTuning.BP_GameTuning_C|GetGoodPortalColor _gamesettings) (Variables|/Game/Blueprints/BP_GameTuning.BP_GameTuning_C|GetBadPortalColor _gamesettings)))))))

(fn ConstructionScript
  (Rendering|SetCastShadow (Variables|Default|GetWidget) false))