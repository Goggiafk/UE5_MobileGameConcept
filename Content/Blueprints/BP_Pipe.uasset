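; A spline-shaped pipe that moves player stickmen from its trigger box to its exit.
; The construction script tiles spline meshes along the spline at scale-based section length and snaps start and end pieces to the first and last points.
; When a "Player"-tagged actor overlaps the box, it is destroyed and BP_StickmenManager spawns a friendly stickman at EndSpawnPoint.
; The manager reference is looked up on actor overlap rather than BeginPlay.
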(event OnComponentBeginOverlap(Box)
  (params (OverlappedComponent :type Primitive%20Component%20Object%20Reference) (OtherActor :type Actor%20Object%20Reference) (OtherComp :type Primitive%20Component%20Object%20Reference) (OtherBodyIndex :type Integer) (bFromSweep :type Boolean) (SweepResult :type Hit%20Result%20Structure%20%28by%20ref%29))
  (bind _stickmenmanager (Variables|Default|GetStickmenManager))
  (Utilities|IsValid OtherActor
    (:Is%20Valid
      (if (Utilities|Array|IsNotEmpty (Variables|/Script/Engine.Actor|GetTags OtherActor))
        (Variables|Default|SetOther%20Actor OtherActor)
        (switch name (Utilities|Array|Get(acopy) (Variables|/Script/Engine.Actor|GetTags (Variables|Default|GetOther%20Actor)))
          (:Stickman
            (if (Actor|ActorHasTag (Variables|Default|GetOther%20Actor) "Player")
              (Utilities|FlowControl|Sequence
                (:then_0
                  (Utilities|IsValid (Variables|Default|GetOther%20Actor)
                    (:Is%20Valid
                      (Actor|DestroyActor (Variables|Default|GetOther%20Actor))
                      (Variables|Default|SetOther%20Actor 0))))
                (:then_1
                  (Utilities|IsValid _stickmenmanager
                    (:Is%20Valid
                      (Default|SpawnStickman _stickmenmanager (Transformation|GetWorldTransform (Variables|Default|GetEndSpawnPoint)) false "None"))))))))))))

(event EventBeginPlay)

(event Collision|EventActorBeginOverlap
  (params (OtherActor :type Actor%20Object%20Reference))
  (bind _returnvalue (Actor|GetActorOfClass "/Game/Blueprints/BP_StickmenManager.BP_StickmenManager_C"))
  (Variables|Default|SetStickmenManager _returnvalue))

(fn ConstructionScript
  (bind _spline (Variables|Default|GetSpline))
  (bind _spline_2 (Variables|Default|GetSpline))
  (bind _spline_3 (Variables|Default|GetSpline))
  (Variables|Default|SetSectionLength (* (.x (Transformation|GetActorScale3D)) 1e+02))
  (Transformation|SetWorldLocation (Variables|Default|GetStartPipe) (Spline|GetLocationatSplinePoint (Variables|Default|GetSpline) 0 "World") false false)
  (for _index (range 0 (Math|Float|Truncate (/ (Spline|GetSplineLength (Variables|Default|GetSpline)) (Variables|Default|GetSectionLength))))
    (Variables|Default|SetLoopIndex _index)
    (bind _returnvalue (AddComponent|AddSplineMeshComponent false))
    (Components|StaticMesh|SetStaticMesh _returnvalue (Variables|Default|GetSplineMesh))
    (SplineMesh|SetForwardAxis _returnvalue "Y" true)
    (SplineMesh|SetStartandEnd _returnvalue (Spline|GetLocationatDistanceAlongSpline _spline_2 (* (Variables|Default|GetLoopIndex) (Variables|Default|GetSectionLength)) "Local") (Spline|GetTangentatDistanceAlongSpline _spline_2 (* (Variables|Default|GetLoopIndex) (Variables|Default|GetSectionLength)) "Local") (Spline|GetLocationatDistanceAlongSpline _spline_3 (* (+ (Variables|Default|GetLoopIndex) 1) (Variables|Default|GetSectionLength)) "Local") (Spline|GetTangentatDistanceAlongSpline _spline_3 (* (+ (Variables|Default|GetLoopIndex) 1) (Variables|Default|GetSectionLength)) "Local") true :!class /Script/Engine.SplineMeshComponent)
    (SplineMesh|SetStartScale _returnvalue "(X=2.000000,Y=2.000000)" true :!class /Script/Engine.SplineMeshComponent)
    (SplineMesh|SetEndScale _returnvalue "(X=2.000000,Y=2.000000)" true :!class /Script/Engine.SplineMeshComponent)
    (Rendering|SetCastShadow _returnvalue false)
    (Rendering|Material|SetMaterial _returnvalue 0 (Variables|Default|GetMaterial)))
  (Transformation|SetWorldLocation (Variables|Default|GetEndPipe) (Spline|GetLocationatSplinePoint _spline (- (Spline|GetNumberOfSplinePoints _spline) 1) "World") false false))