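; BP_StickmenManager spawns player and enemy stickmen and drives their movement from one central actor.
; Each spawn gets a team color and tag, a particle effect and a lifespan from GameSettings, and stays in an array until destroyed.
; A looping timer moves all capsules forward without sweep instead of each stickman ticking.
; Stickmen register with the Animation Sharing Manager to avoid per-character animation cost.
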(event Custom|DestroyLogic
  (params (DestroyedActor :type Actor%20Object%20Reference))
  (Utilities|Array|RemoveItem (Variables|Default|GetStickMen) DestroyedActor))

(event Custom|ProcessStickmenMovement
  (if (Utilities|Array|IsNotEmpty (Variables|Default|GetStickMen))
    (for _array_element (Variables|Default|GetStickMen)
      (Utilities|IsValid _array_element
        (:Is%20Valid
          (Utilities|IsValid (Variables|Default|GetGameSettings)
            (:Is%20Valid
              (Utilities|IsValid (Actor|GetComponentbyClass _array_element "/Script/Engine.CapsuleComponent")
                (:Is%20Valid
                  (Transformation|AddWorldOffset (Actor|GetComponentbyClass _array_element "/Script/Engine.CapsuleComponent") (* (Transformation|GetActorForwardVector _array_element) (Variables|/Game/Blueprints/BP_GameTuning.BP_GameTuning_C|GetStickmenMovementSpeed (Variables|Default|GetGameSettings))) false false))))))))))

(event Custom|SpawnStickman
  (params (Transform :type Transform) (IsEnemy :type Boolean))
  (bind (_location _rotation) (Math|Transform|BreakTransform Transform))
  (bind _gamesettings (Variables|Default|GetGameSettings))
  (bind _returnvalue (Game|SpawnActorfromClass "/Game/Blueprints/BP_Stickman.BP_Stickman_C" (Math|Transform|MakeTransform _location _rotation (Math|Conversions|ToVector(Float) (Variables|/Game/Blueprints/BP_GameTuning.BP_GameTuning_C|GetStickmenSize (Variables|Default|GetGameSettings)))) "AdjustIfPossibleButAlwaysSpawn" "MultiplyWithRoot" 0 0))
  (CallFunction|RegisterStickman _returnvalue)
  (Rendering|Material|SetVectorParameterValueonMaterials (Variables|/Game/Blueprints/BP_Stickman.BP_Stickman_C|GetSkeletalMesh _returnvalue) "Color" (Math|Conversions|ToVector(LinearColor) (select IsEnemy (Variables|/Game/Blueprints/BP_GameTuning.BP_GameTuning_C|GetEnemyStickmenColor _gamesettings) (Variables|/Game/Blueprints/BP_GameTuning.BP_GameTuning_C|GetPlayersStickmenColor _gamesettings))))
  (Utilities|Array|Add (Variables|/Script/Engine.Actor|GetTags _returnvalue) (select IsEnemy (Variables|Default|GetEnemyStickmanTag) (Variables|Default|GetPlayerStickmanTag)))
  (Game|SpawnActorfromClass "/Game/Realistic_Starter_VFX_Pack_Vol2/Blueprints/BP_Spawn_Particle.BP_Spawn_Particle_C" (Math|Transform|MakeTransform (.location (Transformation|GetActorTransform _returnvalue)) (.rotation (Transformation|GetActorTransform _returnvalue)) "0.100000,0.100000,0.100000") "AdjustIfPossibleButAlwaysSpawn" "MultiplyWithRoot" 0 0))

(event Custom|RegisterStickman
  (params (Stickman :type Actor%20Object%20Reference))
  (Utilities|FlowControl|Sequence
    (:then_0
      (Actor|SetLifeSpan Stickman (Variables|/Game/Blueprints/BP_GameTuning.BP_GameTuning_C|GetStickmenLifeSpan (Variables|Default|GetGameSettings)))
      (Utilities|Array|Add (Variables|Default|GetStickMen) Stickman)
      ;[0.15 0.15 0.15 0.5] Retreiving game settings with rules for stickmen
      (Game|BindEventtoOnDestroyed Stickman (delegate Custom|DestroyLogic)))
    (:then_1
      ;[1 1 0] Triggering Shared Animation for each stickman spawned, avoiding costs of animations for separate stickmen
      (bind _returnvalue (Class|AnimationSharingManager|GetAnimationSharingManager))
      (Utilities|IsValid _returnvalue
        (:Is%20Valid
          (Class|AnimationSharingManager|RegisterActorwithSkeletonBP _returnvalue Stickman "/Game/Models/LowPoly_Stickaman_Running_Skeleton.LowPoly_Stickaman_Running_Skeleton"))))))

(event EventBeginPlay
  (bind _returnvalue (Utilities|Time|SetTimerbyEvent (delegate Custom|ProcessStickmenMovement) 0.03 true))
  (Variables|Default|SetMovementTimerHandle _returnvalue))

(fn ConstructionScript)