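; BP_Cannon is the player-controlled cannon that slides sideways and fires stickmen, adding the default Enhanced Input mapping context when possessed.
; Move input offsets it along the control rotation's right vector.
; Shoot input uses DoOnce and a Delay to rate-limit spawns, each delayed stickman being colored, tagged "Player", registered with BP_StickmenManager and given a spawn particle.
; GameSettings drives speed, spawn rate, size and color.
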(event Input|EnhancedActionEvents|EnhancedInputActionIA_Shoot
  (params (ActionValue :type Boolean) (ElapsedSeconds :type Float%20%28double-precision%29) (TriggeredSeconds :type Float%20%28double-precision%29) (InputAction :type Input%20Action%20Object%20Reference :default "/Game/Input/Actions/IA_Shoot.IA_Shoot"))
  (bind _stickmenspawnpoint (Variables|Default|GetStickmenSpawnPoint))
  (bind _returnvalue (Transformation|GetWorldTransform _stickmenspawnpoint))
  (Utilities|FlowControl|DoOnce false :!label _label
    (:Completed
      (Utilities|FlowControl|Delay (- 1.0 (Variables|/Game/Blueprints/BP_GameTuning.BP_GameTuning_C|GetCannonSpawnRate (Variables|Default|GetGameSettings))))
      (bind _returnvalue_2 (Game|SpawnActorfromClass "/Game/Blueprints/BP_Stickman.BP_Stickman_C" (Math|Transform|MakeTransform (.location _returnvalue) (.rotation _returnvalue) (Math|Conversions|ToVector(Float) (Variables|/Game/Blueprints/BP_GameTuning.BP_GameTuning_C|GetStickmenSize (Variables|Default|GetGameSettings)))) "AlwaysSpawn" "MultiplyWithRoot" 0 0))
      (Default|RegisterStickman (Variables|Default|GetStickmenManager) _returnvalue_2)
      (Rendering|Material|SetVectorParameterValueonMaterials (Variables|/Game/Blueprints/BP_Stickman.BP_Stickman_C|GetSkeletalMesh _returnvalue_2) "Color" (Math|Conversions|ToVector(LinearColor) (Variables|/Game/Blueprints/BP_GameTuning.BP_GameTuning_C|GetPlayersStickmenColor (Variables|Default|GetGameSettings))))
      (Utilities|Array|Add (Variables|/Script/Engine.Actor|GetTags _returnvalue_2) "Player")
      (Game|SpawnActorfromClass "/Game/Realistic_Starter_VFX_Pack_Vol2/Blueprints/BP_Spawn_Particle.BP_Spawn_Particle_C" (Transformation|GetActorTransform _returnvalue_2) "Undefined" "MultiplyWithRoot" 0 0)
      (goto _label Reset))))

(event Input|EnhancedActionEvents|EnhancedInputActionIA_Move
  (params (ActionValue :type Float%20%28double-precision%29) (ElapsedSeconds :type Float%20%28double-precision%29) (TriggeredSeconds :type Float%20%28double-precision%29) (InputAction :type Input%20Action%20Object%20Reference :default "/Game/Input/Actions/IA_Move.IA_Move"))
  (bind _returnvalue (Pawn|GetControlRotation :!class /Script/Engine.Pawn))
  (Transformation|SetActorLocation self (+ (Transformation|GetActorLocation) (* (Math|Vector|GetRightVector (Math|Rotator|MakeRotator (.roll _returnvalue) 0.0 (.yaw _returnvalue))) (* ActionValue (Variables|/Game/Blueprints/BP_GameTuning.BP_GameTuning_C|GetCannonMovementSpeed (Variables|Default|GetGameSettings))))) false false))

(event EventBeginPlay
  (bind _returnvalue (Actor|GetActorOfClass "/Game/Blueprints/BP_StickmenManager.BP_StickmenManager_C"))
  (Variables|Default|SetStickmenManager _returnvalue))

(event EventControllerChanged
  (params (OldController :type Controller%20Object%20Reference) (NewController :type Controller%20Object%20Reference))
  (bind _asplayer_controller (Utilities|Casting|CastToPlayerController NewController))
  (Input|AddMappingContext (PlayerController|LocalPlayerSubsystems|GetEnhancedInputLocalPlayerSubsystem _asplayer_controller) "/Game/Input/IMC_Default.IMC_Default" 0 "(bIgnoreAllPressedKeysUntilRelease=True,bForceImmediately=False,bNotifyUserSettings=False)"))

(fn ConstructionScript)