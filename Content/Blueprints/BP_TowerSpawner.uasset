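; BP_TowerSpawner periodically spawns waves of enemy stickmen at its spawn point.
; On BeginPlay it finds the BP_StickmenManager and starts a looping timer at the tower spawn rate from GameSettings.
; Each tick of that timer asks the manager to spawn a batch of enemies.
; When GameSettings enables increasing counts, the batch size scales linearly with the number of waves so far.
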(event Custom|SpawnEnemies
  (bind _gamesettings (Variables|Default|GetGameSettings))
  (bind _spawncount (Variables|/Game/Blueprints/BP_GameTuning.BP_GameTuning_C|GetSpawnCount _gamesettings))
  (Math|Integer|IncrementInt (Variables|Default|GetSpawnLoops)
    (:%20%20
      (for _index (range 0 (select (Variables|/Game/Blueprints/BP_GameTuning.BP_GameTuning_C|GetShouldSpawnCountIncrease? _gamesettings) (* _spawncount (Variables|Default|GetSpawnLoops)) _spawncount))
        (Default|SpawnStickman (Variables|Default|GetStickmenManager) (Transformation|GetWorldTransform (Variables|Default|GetSpawnPoint)) true)))))

(event EventBeginPlay
  (bind _returnvalue (Actor|GetActorOfClass "/Game/Blueprints/BP_StickmenManager.BP_StickmenManager_C"))
  (Variables|Default|SetStickmenManager _returnvalue)
  (bind _returnvalue_2 (Utilities|Time|SetTimerbyEvent (delegate Custom|SpawnEnemies) (Variables|/Game/Blueprints/BP_GameTuning.BP_GameTuning_C|GetTowerSpawnRate (Variables|Default|GetGameSettings)) true))
  (Variables|Default|SetSpawnEnemiesTimeHandle _returnvalue_2))

(fn ConstructionScript)